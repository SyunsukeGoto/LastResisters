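; BP_Enemy2 is an enemy that dissolves in near the player, chases and attacks, then returns to its spawn point and fades out when out of range.
; Tick drives an enum state machine, mirroring state and target location to the Blackboard.
; Mesh overlaps damage and knock back the player, while raised-shield hits drain Block toward a downed state.
; It also updates its HP/Block widget, barrier visibility and floating damage numbers.
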(event `self.ReceiveBeginPlay`
  (bind _output_get (set `self.Enemy1State` "NewEnumerator6"))
  (`BlackboardComponent.SetValueAsEnum` (`AIBlueprintHelperLibrary.GetBlackboard` self) (`KismetStringLibrary.Conv_StringToName` "states") _output_get)
  (`MeshComponent.SetScalarParameterValueOnMaterials` (`self.Mesh`) "Amount" 2.5)
  (set `self.TownPos` (`SceneComponent.K2_GetComponentLocation` (`self.Mesh`)))
  (bind _asmy_game_instance (cast `MyGameInstance` (`GameplayStatics.GetGameInstance`)))
  (bind _returnvalue (`MyGameInstance.GetPlayerHp` _asmy_game_instance))
  (bind _asbp_new_enemy_ui (cast `/Game/Game/UI/In_Game/EnemyUI/Blueprints/BP_NewEnemyUI` (`WidgetComponent.GetUserWidgetObject` (`self.Widget`))))
  (`MeshComponent.SetScalarParameterValueOnMaterials` (`self.baria`) "Opacity" -20.0))

(event `self.ReceiveActorBeginOverlap`
  (params (OtherActor :type "Actor Object Reference")))

(event `self.ReceiveTick`
  (params (DeltaSeconds :type "Float (single-precision)"))
  (`|ExecutionSequence`
    (:`then_0`
      (`self.StateLoppStates`))
    (:`then_1`
      (`self.UpdateBlackBoardStates`))
    (:`then_2`
      (`self.AttackDistanceEvente`))
    (:`then_3`
      (`self.PlayerDistanceSpawn`))
    (:`then_4`
      (if (`|EnumEquality` (`self.Enemy1State`) "NewEnumerator9")
        (`self.GoToTown`)))
    (:`then_5`
      (`self.BariaAndHart`))
    (:`then_6`
      (if (`|EnumEquality` (`self.Enemy1State`) "NewEnumerator8")
        (`self.AttackEvent`)
        (else
          (`self.PlayerDistanceSpawn`))))
    (:`then_7`
      (if (`|EnumEquality` (`self.Enemy1State`) "NewEnumerator9")
        (`self.PeceOutDistance`)))
    (:`then_8`
      (set `/Game/Game/UI/In_Game/EnemyUI/Blueprints/BP_NewEnemyUI.EnemyHP` (`self.Hp`) (stale `self.ReceiveBeginPlay` _asbp_new_enemy_ui))
      (set `/Game/Game/UI/In_Game/EnemyUI/Blueprints/BP_NewEnemyUI.EnemyBlock` (`self.Block`) (stale `self.ReceiveBeginPlay` _asbp_new_enemy_ui)))
    (:`then_9`
      (`self.DefencedEvent`))
    (:`then_10`
      (`self.DownEvent`))
    (:`then_11`
      (if (`|EnumEquality` (`self.Enemy1State`) "NewEnumerator8")
        _))
    (:`then_12`
      (`self.RotToPlayer`))
    (:`then_13`
      (if (<= (`self.Hp`) 0)
        (set `self.Hp` 0)
        (set `self.Enemy1State` "NewEnumerator11")))
    (:`then_14`
      ;[1 1 1] ダメージ数を表示するオブジェクトを生成する
      (if (`self.DamagedFlag`)
        (bind _returnvalue (`|SpawnActorFromClass` "/Game/Game/Blueprints/DamageNumber/BP_DamargeNumber.BP_DamargeNumber_C" (`SceneComponent.K2_GetComponentToWorld` (`self.DamageNumberPos`)) "Undefined" "OverrideRootScale" null null))
        (set `/Game/Game/Blueprints/DamageNumber/BP_DamargeNumber.TextNum` (`KismetTextLibrary.Conv_IntToText` (`self.DamagedNum`)) _returnvalue)
        (set `/Game/Game/Blueprints/DamageNumber/BP_DamargeNumber.Color` (`self.Color`) _returnvalue)
        (set `self.DamagedFlag` false)))))

(event `DownEvent`
  ;[1 1 1] ダウンした時の立ち上がる処理
  (if (`|EnumEquality` (`self.Enemy1State`) "NewEnumerator5")
    (set `self.Block` 100)
    (elif (<= (`self.Block`) 0)
      (set `self.Enemy1State` "NewEnumerator4"))))

(event `BariaAndHart`
  (bind _baria (`self.baria`))
  ;[1 1 1] バリアと心臓の描画処理
  (if (`|EnumEquality` (`self.Enemy1State`) "NewEnumerator6")
    (`SceneComponent.SetVisibility` (`self.Cube`) true false)
    (`SceneComponent.SetVisibility` (`self.baria`) false false)
    (else
      (`SceneComponent.SetVisibility` (`self.Cube`) false false)
      (if (`|EnumInequality` (`self.Enemy1State`) "NewEnumerator4")
        (`SceneComponent.SetVisibility` _baria true false)
        (else
          (`SceneComponent.SetVisibility` _baria false false))))))

(event `SpawnEvent`
  ;[1 1 1] 敵の出現処理
  (bind (_direction _newtrack_0) (`Timeline|spanwTimeLine` :!via `PlayFromStart`)
    (:`Update`
      (`MeshComponent.SetScalarParameterValueOnMaterials` (`self.Mesh`) "Amount" _newtrack_0))))

(event `RotToPlayer`
  (bind (_returnvalue_roll _returnvalue_pitch _returnvalue_yaw) (`KismetMathLibrary.BreakRotator` (`KismetMathLibrary.RInterpTo` (`self.K2_GetActorRotation`) (`KismetMathLibrary.FindLookAtRotation` (`self.K2_GetActorLocation`) (`self.K2_GetActorLocation` (`GameplayStatics.GetPlayerPawn` 0))) (`GameplayStatics.GetWorldDeltaSeconds`) 2.0)))
  ;[1 1 1] 方向をプレイヤーに向ける処理
  (`self.K2_SetActorRotation` (`KismetMathLibrary.MakeRotator` 0.0 0.0 _returnvalue_yaw)))

(event `KillRob`
  ;[1 1 1] 死んだときの処理
  (`self.K2_DestroyActor`)
  (`GameplayStatics.SpawnEmitterAtLocation` "/Game/StarterContent/Particles/P_Explosion.P_Explosion" (`self.K2_GetActorLocation`) (struct) (50.0 50.0 50.0)))

(event `PeaceOutEvent`
  ;[1 1 1] 敵が消える処理
  (bind (_direction _newtrack_0) (`Timeline|PeaceOutTimeLine` :!via `PlayFromStart`)
    (:`Update`
      (`MeshComponent.SetScalarParameterValueOnMaterials` (`self.Mesh`) "Amount" (* _newtrack_0 -1.0)))))

(event `AttackEvent`
  (bind _returnvalue (`KismetMathLibrary.RandomInteger` 2))
  (bind _attackdistance (`self.AttackDistance`))
  (bind _returnvalue_2 (`KismetMathLibrary.Vector_Distance` (`self.K2_GetActorLocation` (`GameplayStatics.GetPlayerPawn` 0)) (`self.K2_GetActorLocation`)))
  ;[1 1 1] 攻撃処理
  (if (<= _returnvalue_2 _attackdistance)
    (if (<= _returnvalue_2 (- _attackdistance 110.0))
      ;[1 1 1] 攻撃距離かの計算処理
      (`self.LaunchCharacter` (`GameplayStatics.GetPlayerCharacter` 0) (* (`self.GetActorForwardVector`) 70.0) false false :!label _label)
      (elif (== _returnvalue 0)
        (set `self.Enemy1State` "NewEnumerator1")
        (elif (== _returnvalue 1)
          (set `self.Enemy1State` "NewEnumerator2")
          (else
            (if (== _returnvalue 2)
              _
              (else
                _))
            (set `self.Enemy1State` "NewEnumerator2")))))
    (else
      (set `self.Enemy1State` "NewEnumerator0"))))

(event `FindPlayerPOsition`
  (bind _attackangle (`self.AttackAngle`))
  ;[1 1 1] プレイヤーの位置を探す処理
  (`BlackboardComponent.SetValueAsVector` (`AIBlueprintHelperLibrary.GetBlackboard` self) (`KismetStringLibrary.Conv_StringToName` "TargetLocation") (+ (`NavigationSystemV1.K2_GetRandomLocationInNavigableRadius` (`self.K2_GetActorLocation` (`GameplayStatics.GetPlayerPawn` 0)) 0.0 null null) (`KismetMathLibrary.MakeVector` (* (`KismetMathLibrary.Cos` _attackangle) 140.0) (* (`KismetMathLibrary.Sin` _attackangle) 140.0)))))

(event `AttackDistanceEvente`
  (bind _attackdistance (`self.AttackDistance`))
  (bind _returnvalue (`KismetMathLibrary.Vector_Distance` (`self.K2_GetActorLocation` (`GameplayStatics.GetPlayerPawn` 0)) (`self.K2_GetActorLocation`)))
  ;[1 1 1] 攻撃距離かの計算処理
  (if (`|EnumEquality` (`self.Enemy1State`) "NewEnumerator0")
    (if (<= _returnvalue _attackdistance)
      (set `self.Enemy1State` "NewEnumerator8")
      (if (<= _returnvalue (- _attackdistance 95.0))
        (goto _label)))))

(event `StateLoppStates`
  ;[1 1 1] 攻撃距離かの計算処理
  (if (`|EnumEquality` (`self.Enemy1State`) "NewEnumerator0")
    (`self.FindPlayerPOsition`)
    (elif (`|EnumEquality` (`self.Enemy1State`) "NewEnumerator7")
      (`self.SpawnEvent`)
      (set `self.Enemy1State` "NewEnumerator0"))))

(event `UpdateBlackBoardStates`
  ;[1 1 1] ブラックボードの状態の更新処理
  (`BlackboardComponent.SetValueAsEnum` (`AIBlueprintHelperLibrary.GetBlackboard` self) (`KismetStringLibrary.Conv_StringToName` "states") (`self.Enemy1State`)))

(event `PlayerDistanceSpawn`
  (bind _returnvalue (`|EnumEquality` (`self.Enemy1State`) "NewEnumerator6"))
  ;[1 1 1] プレイヤー出現距離計算処理
  (if (< (`KismetMathLibrary.Vector_Distance` (`self.K2_GetActorLocation` (`GameplayStatics.GetPlayerPawn` 0)) (`self.K2_GetActorLocation`)) (`self.SpawnDistance`))
    (if _returnvalue
      (set `self.Enemy1State` "NewEnumerator7"))
    (elif (not _returnvalue)
      (set `self.Enemy1State` "NewEnumerator9"))))

(event `DefencedEvent`
  ;[1 1 1] 守備処理
  (if (`self.DefecedFlag`)
    (if (>= (`self.DefenceCount`) 40)
      (set `self.DefecedFlag` false)
      (set `self.DefenceCount` 0)
      (else
        (set `self.DefenceCount` (+ (`self.DefenceCount`) 1))))))

(event `PeceOutDistance`
  ;[1 1 1] 敵が消える距離化の計算処理
  (if (< (`KismetMathLibrary.Vector_Distance` (`self.TownPos`) (`SceneComponent.K2_GetComponentLocation` (`self.Mesh`))) (`self.AttackDistance`))
    (`self.PeaceOutEvent`)
    (set `self.Enemy1State` "NewEnumerator6")))

(event `GoToTown`
  ;[1 1 1] 元の場所を探す処理
  (`BlackboardComponent.SetValueAsVector` (`AIBlueprintHelperLibrary.GetBlackboard` self) (`KismetStringLibrary.Conv_StringToName` "TargetLocation") (`NavigationSystemV1.K2_GetRandomLocationInNavigableRadius` (`self.TownPos`) 0.0 null null)))

(event `self.Mesh.OnComponentBeginOverlap`
  (params (OverlappedComponent :type "PrimitiveComponent Object Reference") (OtherActor :type "Actor Object Reference") (OtherComp :type "PrimitiveComponent Object Reference") (OtherBodyIndex :type Integer) (bFromSweep :type Boolean) (SweepResult :type "HitResult Structure (by ref)"))
  (bind _returnvalue (`GameplayStatics.GetPlayerCharacter` 0))
  (bind _returnvalue_2 (`self.GetActorForwardVector` (`GameplayStatics.GetPlayerPawn` 0)))
  ;[1 1 1] プレイヤーとの当たり判定
  (if (`ActorComponent.ComponentHasTag` OtherComp "Player")
    (if (`|EnumEquality` (`self.Enemy1State`) "NewEnumerator1")
      (bind _asmy_game_instance (cast `MyGameInstance` (`GameplayStatics.GetGameInstance`) :!label _label_2))
      (if (not (`self.DefecedFlag`))
        (`MyGameInstance.DamageToPlayer` _asmy_game_instance 2.0)
        (if (`|EnumEquality` (`self.Enemy1State`) "NewEnumerator1")
          (`self.LaunchCharacter` _returnvalue (* _returnvalue_2 -70.0) false false))
        (`GameplayStatics.PlaySoundAtLocation` "/Game/Game/Sound/SE/hit01__online-audio-converter_com_.hit01__online-audio-converter_com_" _returnvalue_2 (struct) 1.0 1.0 0.0 null null null)
        (bind _asmotion_controller_pawn (cast `/Game/VirtualRealityBP/Blueprints/MotionControllerPawn` _returnvalue))
        (set `/Game/VirtualRealityBP/Blueprints/MotionControllerPawn.SaveMeFlag` true _asmotion_controller_pawn)
        (set `/Game/VirtualRealityBP/Blueprints/MotionControllerPawn.SaveMeCount` 0 _asmotion_controller_pawn)
        (set `MyGameInstance.damageTaken` (+ (`MyGameInstance.damageTaken` _asmy_game_instance) 5.0) _asmy_game_instance))
      (elif (`|EnumEquality` (`self.Enemy1State`) "NewEnumerator2")
        (goto _label_2)
        (elif (`|EnumEquality` (`self.Enemy1State`) "NewEnumerator3")
          (goto _label_2))))
    (elif (`ActorComponent.ComponentHasTag` OtherComp "Shield")
      (bind _asbp_shield (cast `/Game/Game/Weapons/BP/BP_Shield` OtherActor))
      (if (`/Game/Game/Weapons/BP/BP_Shield.UseShieldFlag` _asbp_shield)
        (if (`self.DefecedFlag`)
          _
          (elif (`|EnumEquality` (`self.Enemy1State`) "NewEnumerator1")
            (set `self.DefecedFlag` true :!label _label_3)
            (set `self.Block` (- (`self.Block`) 30))
            (elif (`|EnumEquality` (`self.Enemy1State`) "NewEnumerator2")
              (goto _label_3)
              (elif (`|EnumEquality` (`self.Enemy1State`) "NewEnumerator3")
                (goto _label_3)))))))))

(event `RandomAttackAngle`
  (bind (_returnvalue_roll _returnvalue_pitch _returnvalue_yaw) (`KismetMathLibrary.BreakRotator` (`self.K2_GetActorRotation` (`GameplayStatics.GetPlayerPawn` 0))))
  (`self.LaunchCharacter` (* (`self.GetActorForwardVector`) -700.0))
  (set `self.Enemy1State` "NewEnumerator0")
  (if (== (`KismetMathLibrary.FFloor64` (`self.AttackAngle`)) 0)
    (switch `int` (`KismetMathLibrary.RandomIntegerInRange` 0 2)
      (:`Default`
        (set `self.AttackAngle` _returnvalue_yaw :!label _label_4))
      (:`0`
        (goto _label_4))
      (:`1`
        (set `self.AttackAngle` (+ _returnvalue_yaw 45.0)))
      (:`2`
        (set `self.AttackAngle` (+ _returnvalue_yaw -45.0))))
    (else
      (goto _label_4))))

(fn `GetDefenceFlag`
  (returns (NewParam :type Boolean))
  (return (`self.DefecedFlag`)))

(fn `UserConstructionScript`)