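; A floating damage number actor that displays a value as world text, drifts vertically and then removes itself.
; On BeginPlay the DestroyTime timeline plays and destroys the actor when finished.
; Each Tick sets the text and color from variables and rotates the actor to face the player camera.
; Tick also zeroes the movement vector's X and Y, scales Z by a constant for frame-rate-dependent acceleration, and offsets the root by it.
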(event `self.ReceiveBeginPlay`
  (`Timeline|DestroyTime`
    (:`Finished`
      (`self.K2_DestroyActor`))))

(event `self.ReceiveTick`
  (params (DeltaSeconds :type "Float (single-precision)"))
  (bind _vector (`self.Vector`))
  (`|ExecutionSequence`
    (:`then_0`
      (`TextRenderComponent.K2_SetText` (`self.TextRender`) (`self.TextNum`))
      (`self.K2_SetActorRotation` (`KismetMathLibrary.FindLookAtRotation` (`self.K2_GetActorLocation`) (`PlayerCameraManager.GetCameraLocation` (`GameplayStatics.GetPlayerCameraManager` 0))))
      (`TextRenderComponent.SetTextRenderColor` (`self.TextRender`) (`self.Color`)))
    (:`then_1`
      (set `self.Vector` (* _vector (0.0 0.0 1.3))))
    (:`then_2`
      (`SceneComponent.K2_AddRelativeLocation` (`self.DefaultSceneRoot`) _vector false false))))

(fn `UserConstructionScript`)