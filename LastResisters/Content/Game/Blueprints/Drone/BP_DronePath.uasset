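; BP_DronePath is the drone's spline path actor, which follows the VR headset and keeps itself in front of the player.
; On BeginPlay it spawns a BP_Drone, passes itself as the path reference and attaches the drone.
; Each Tick it moves to a set distance along the camera's forward vector, offset by HMD position, with Z fixed at Height.
; It takes yaw and roll from a look-at rotation toward the camera.
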(event `self.ReceiveTick`
  (params (DeltaSeconds :type "Float (single-precision)"))
  (bind _returnvalue (`GameplayStatics.GetPlayerCameraManager` 0))
  (bind _returnvalue_2 (`self.K2_GetActorLocation` _returnvalue))
  (bind (_returnvalue_roll _returnvalue_pitch _returnvalue_yaw) (`KismetMathLibrary.BreakRotator` (`KismetMathLibrary.FindLookAtRotation` (`self.K2_GetActorLocation`) _returnvalue_2)))
  (bind (_returnvalue_x _returnvalue_y) (`KismetMathLibrary.BreakVector` (+ (* (`KismetMathLibrary.GetForwardVector` (`self.K2_GetActorRotation` _returnvalue)) (`self.DistFromPlayer`)) (+ _returnvalue_2 (`.DevicePosition` (`HeadMountedDisplayFunctionLibrary.GetOrientationAndPosition`))))))
  ;[1 1 1] Set the drone spline to follow the HMD position. Z-axis can be adjusted by changing the Height variable value
  (`self.K2_SetActorLocationAndRotation` (`KismetMathLibrary.MakeVector` _returnvalue_x _returnvalue_y (`self.Height`)) (`KismetMathLibrary.MakeRotator` _returnvalue_roll 0.0 _returnvalue_yaw)))

(event `self.ReceiveBeginPlay`
  ;[1 1 1] Spawn and attach the drone
  (bind _returnvalue (`|SpawnActorFromClass` "/Game/Game/Blueprints/Drone/BP_Drone.BP_Drone_C" (`self.GetTransform`) "Undefined" "OverrideRootScale" null self null))
  (`self.K2_AttachToActor` _returnvalue self "None" "KeepRelative" "KeepRelative" "KeepRelative" true))

(fn `UserConstructionScript`)