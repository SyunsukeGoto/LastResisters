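; BP_WarpPoint is a warp point actor that detects when the VR player reaches its particle effect.
; Every Tick it stores the horizontal distance, ignoring height, between the particle system and the MotionControllerPawn's mesh.
; It sets WarpFlag once that distance drops below a fixed radius; this graph neither clears the flag nor performs the warp.
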(event `self.ReceiveTick`
  (params (DeltaSeconds :type "Float (single-precision)"))
  (bind (_returnvalue_x _returnvalue_y) (`KismetMathLibrary.BreakVector` (`SceneComponent.K2_GetComponentLocation` (`self.ParticleSystem`))))
  (bind (_returnvalue_x_2 _returnvalue_y_2) (`KismetMathLibrary.BreakVector` (`SceneComponent.K2_GetComponentLocation` (`Character.Mesh` (cast `/Game/VirtualRealityBP/Blueprints/MotionControllerPawn` (`GameplayStatics.GetPlayerPawn` 0) :!pure true)))))
  (bind _returnvalue (`KismetMathLibrary.Abs` (`KismetMathLibrary.VSize` (- (`KismetMathLibrary.MakeVector` _returnvalue_x _returnvalue_y) (`KismetMathLibrary.MakeVector` _returnvalue_x_2 _returnvalue_y_2)))))
  (set `self.PlauerDistance` _returnvalue)
  (if (< _returnvalue 75.0)
    (set `self.WarpFlag` true)))

(fn `UserConstructionScript`)