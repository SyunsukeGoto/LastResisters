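; BP_EnemyShield_TypeB is an enemy shield actor that lights up when hit and shatters when broken.
; BeginPlay puts a dynamic material on the shield, and HIT plays the LightUp timeline to drive its emissive and opacity.
; Break runs once, darkening the shield, brightening and fracturing the DmPlane destructible through ApplyDamage, then destroying the actor after a timeline.
; Space and Backspace keys act as test triggers.
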(event `self.ReceiveBeginPlay`
  (bind _returnvalue (`KismetMaterialLibrary.CreateDynamicMaterialInstance` "/Game/Game/Material/EnemyShieldMaterial/M_DefaultEnemyShield.M_DefaultEnemyShield"))
  (bind _output_get (set `self.ShiledMatetrial` _returnvalue))
  (`PrimitiveComponent.SetMaterial` (`self.shield`) 0 _output_get)
  (`MeshComponent.SetScalarParameterValueOnMaterials` (`self.dm_plane`) "Emisive" (`self.AplhaMinValue`)))

(event `HIT`
  ;[1 1 1] Hit
  (bind (_direction _newtrack_0) (`Timeline|LightUp` :!via `PlayFromStart` :!label _label)
    (:`Update`
      (`MeshComponent.SetScalarParameterValueOnMaterials` (`self.shield`) "Emisive" _newtrack_0)
      (`MeshComponent.SetScalarParameterValueOnMaterials` (`self.shield`) "Opacity" _newtrack_0))))

(event `Key|SpaceBar`
  (params (Key :type "Key Structure"))
  ;[1 1 1] Test
  (:`Pressed`
    (goto _label :!via `PlayFromStart`)))

(event `Break`
  (bind _dm_plane (`self.dm_plane`))
  ;[1 1 1] ShieldBreak
  (`/Engine/EditorBlueprintResources/StandardMacros.DoOnce` false :!label _label_2
    (:`Completed`
      (`MeshComponent.SetScalarParameterValueOnMaterials` (`self.shield`) "Emisive" 0.0)
      (`DestructibleComponent.ApplyDamage` _dm_plane 10.0 (`SceneComponent.K2_GetComponentLocation` _dm_plane) (1.0 0.0 0.0) 500.0)
      (`MeshComponent.SetScalarParameterValueOnMaterials` (`self.dm_plane`) "Emisive" (`self.AlphaMaxValue`))
      (`Timeline|Timeline_0` :!via `PlayFromStart`
        (:`Finished`
          (`self.K2_DestroyActor`))))))

(event `Key|BackSpace`
  (params (Key :type "Key Structure"))
  ;[1 1 1] Test
  (:`Pressed`
    (goto _label_2)))

(fn `UserConstructionScript`)