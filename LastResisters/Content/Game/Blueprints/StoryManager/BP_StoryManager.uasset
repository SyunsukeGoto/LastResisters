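; Story manager actor that presents a sequence of story messages through a hovering drone and a world-space text widget.
; Drone bobs on a timeline and faces the player, while it and the widget track camera height.
; After a delayed intro animation, MessegeButton steps through three-line text arrays, animating description textures for flagged messages.
; DoOnce gates refresh the widget per message, and pressing on the last one sets the story-finished flag.
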(event `self.ReceiveBeginPlay`
  (bind _asui_story_messege (cast `/Game/Game/UI/In_Game/StoryMessege/UI_StoryMessege` (`WidgetComponent.GetUserWidgetObject` (`self.MessegeText`)) :!pure true))
  (`|ExecutionSequence`
    (:`then_0`
      (`KismetSystemLibrary.Delay` 1.0)
      (`SceneComponent.SetHiddenInGame` (`self.MessegeText`) false false)
      (`UserWidget.PlayAnimation` _asui_story_messege (`/Game/Game/UI/In_Game/StoryMessege/UI_StoryMessege.OpenMessegeWindow` _asui_story_messege) 0.0 1 "Forward" 1.0)
      (`KismetSystemLibrary.Delay` 1.0)
      (set `self.StoryStartFlag` true))))

(event `self.ReceiveTick`
  (params (DeltaSeconds :type "Float (single-precision)"))
  (bind _drone (`self.Drone`))
  (bind _messegecount (`self.MessegeCount`))
  (bind _messegetext (`self.MessegeText`))
  (bind _drone_2 (`self.Drone`))
  (bind (_returnvalue_x _returnvalue_y _returnvalue_z) (`KismetMathLibrary.BreakVector` (`self.K2_GetActorLocation` (`GameplayStatics.GetPlayerCameraManager` 0))))
  (bind (_returnvalue_x_2 _returnvalue_y_2) (`KismetMathLibrary.BreakVector` (`SceneComponent.K2_GetComponentLocation` _drone)))
  (bind (_returnvalue_x_3 _returnvalue_y_3 _returnvalue_z_2) (`KismetMathLibrary.BreakVector` (`self.K2_GetActorLocation` (`GameplayStatics.GetPlayerCameraManager` 0))))
  (bind (_returnvalue_x_4 _returnvalue_y_4) (`KismetMathLibrary.BreakVector` (`SceneComponent.K2_GetComponentLocation` _messegetext)))
  (bind _asui_story_messege (cast `/Game/Game/UI/In_Game/StoryMessege/UI_StoryMessege` (`WidgetComponent.GetUserWidgetObject` (`self.MessegeText`)) :!pure true))
  (bind _asui_story_messege_2 (cast `/Game/Game/UI/In_Game/StoryMessege/UI_StoryMessege` (`WidgetComponent.GetUserWidgetObject` (`self.MessegeText`)) :!pure true))
  (`|ExecutionSequence`
    (:`then_0`
      ;[1 1 1] DroneHoverMove
      (`/Engine/EditorBlueprintResources/StandardMacros.DoOnce` false :!label _label
        (:`Completed`
          (bind (_direction _hovemove) (`Timeline|DroneHoverMove` :!via `PlayFromStart`)
            (:`Update`
              (`SceneComponent.K2_SetWorldLocation` _drone (`KismetMathLibrary.MakeVector` _returnvalue_x_2 _returnvalue_y_2 (+ (* _hovemove (`self.HovePower`)) (+ _returnvalue_z (`self.DronePos`)))) false false))
            (:`Finished`
              (goto _label :!via `Reset`))))))
    (:`then_1`
      (`SceneComponent.K2_SetWorldRotation` _drone_2 (`KismetMathLibrary.FindLookAtRotation` (`SceneComponent.K2_GetComponentLocation` _drone_2) (`self.K2_GetActorLocation` (`GameplayStatics.GetPlayerPawn` 0))) false false))
    (:`then_2`
      ;[1 1 1] MessegeText
      (if (== (`self.StoryStartFlag`) true)
        (`/Engine/EditorBlueprintResources/StandardMacros.DoOnce` false :!label _label_2
          (:`Completed`
            (set `/Game/Game/UI/In_Game/StoryMessege/UI_StoryMessege.MessegeLine1` (`KismetTextLibrary.Conv_StringToText` (`|GetArrayItem` (`self.StoryLine1Text`) _messegecount)) _asui_story_messege_2)
            (set `/Game/Game/UI/In_Game/StoryMessege/UI_StoryMessege.MessegeLine2` (`KismetTextLibrary.Conv_StringToText` (`|GetArrayItem` (`self.StoryLine2Text`) _messegecount)) _asui_story_messege_2)
            (set `/Game/Game/UI/In_Game/StoryMessege/UI_StoryMessege.MessegeLine3` (`KismetTextLibrary.Conv_StringToText` (`|GetArrayItem` (`self.StoryLine3Text`) _messegecount)) _asui_story_messege_2)))))
    (:`then_3`
      ;[1 1 1] MessegeUILocation
      (`SceneComponent.K2_SetWorldLocation` _messegetext (`KismetMathLibrary.MakeVector` _returnvalue_x_4 _returnvalue_y_4 (+ (`self.MessegePosZ`) _returnvalue_z_2)) false false))
    (:`then_4`
      (if (== (`|GetArrayItem` (`self.UseTextureFlag`) (`self.MessegeCount`)) true)
        (`/Engine/EditorBlueprintResources/StandardMacros.DoOnce` false :!label _label_3
          (:`Completed`
            (if (!= (`self.MessegeCount`) (`self.MAX_MESSEGE`))
              (set `/Game/Game/UI/In_Game/StoryMessege/UI_StoryMessege.NowTextureIndex` (`self.MessegeCount`) _asui_story_messege :!label _label_4)
              (`UserWidget.PlayAnimation` _asui_story_messege (`/Game/Game/UI/In_Game/StoryMessege/UI_StoryMessege.OpenDescriptiontexture` _asui_story_messege) 0.0 1 "Forward" 1.0)
              (elif (== (`self.MessegeCount`) (`self.MAX_MESSEGE`))
                (goto _label_4)))))))))

(event `InputAction|MessegeButton`
  (params (Key :type "Key Structure"))
  (bind _asui_story_messege (cast `/Game/Game/UI/In_Game/StoryMessege/UI_StoryMessege` (`WidgetComponent.GetUserWidgetObject` (`self.MessegeText`)) :!pure true))
  (:`Pressed`
    ;[1 1 1] MessegeText
    (if (== (`self.StoryStartFlag`) true)
      (if (!= (`self.MessegeCount`) (`self.MAX_MESSEGE`))
        (`|ExecutionSequence`
          (:`then_0`
            (if (== (`|GetArrayItem` (`self.UseTextureFlag`) (`self.MessegeCount`)) true) :!label _label_5
              (`UserWidget.PlayAnimation` _asui_story_messege (`/Game/Game/UI/In_Game/StoryMessege/UI_StoryMessege.CloseDesciptiontexture` _asui_story_messege) 0.0 1 "Forward" 1.0)
              (`KismetSystemLibrary.Delay` 1.0)
              (goto _label_3 :!via `Reset`)
              (else
                (goto _label_3 :!via `Reset`))))
          (:`then_1`
            (set `self.MessegeCount` (+ (`self.MessegeCount`) 1))
            (goto _label_2 :!via `Reset`)))
        (else
          (`|ExecutionSequence`
            (:`then_0`
              (`/Engine/EditorBlueprintResources/StandardMacros.DoOnce` false
                (:`Completed`
                  (set `self.StoryFnishFlag` true))))
            (:`then_1`
              (goto _label_5))))))))

(fn `UserConstructionScript`)