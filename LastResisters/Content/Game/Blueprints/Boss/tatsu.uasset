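; Behavior tree task that runs the boss's tornado attack when its TatsuFlag is set, and finishes successfully at once otherwise.
; Above 50 HP one tornado eases forward; at 50 or below, three launch together in a faster, shorter spread.
; Each is shown, moved by MoveComponentTo to an offset from the capsule's world location, snapped back and hidden.
; The attack then clears the flag and finishes as failed.
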(event `self.ReceiveExecuteAI`
  (params (OwnerController :type "AIController Object Reference") (ControlledPawn :type "Pawn Object Reference"))
  (bind _asbp_boss (cast `/Game/Game/Blueprints/Boss/BP_Boss` ControlledPawn))
  (if (`/Game/Game/Blueprints/Boss/BP_Boss.TatsuFlag` _asbp_boss)
    (if (<= (`/Game/Game/Blueprints/Boss/BP_Boss.Hp` _asbp_boss) 50)
      (`|ExecutionSequence`
        (:`then_0`
          (bind _p_tornado2 (`/Game/Game/Blueprints/Boss/BP_Boss.P_Tornado2` _asbp_boss))
          (`SceneComponent.SetVisibility` _p_tornado2 true false)
          (bind _capsulecomponent (`Character.CapsuleComponent` _asbp_boss))
          (`KismetSystemLibrary.MoveComponentTo` _p_tornado2 (+ (`SceneComponent.K2_GetComponentLocation` _capsulecomponent) (1000.0 -1000.0 0.0)) (struct) false false 1.0)
          (bind _returnvalue (+ (`SceneComponent.K2_GetComponentLocation` _capsulecomponent) (1500.0 0.0 -200.0)))
          (`KismetSystemLibrary.MoveComponentTo` _p_tornado2 _returnvalue (struct) false false 0.0)
          (`SceneComponent.SetVisibility` _p_tornado2 false false))
        (:`then_1`
          (bind _p_tornado1 (`/Game/Game/Blueprints/Boss/BP_Boss.P_Tornado1` _asbp_boss))
          (`SceneComponent.SetVisibility` _p_tornado1 true false)
          (`KismetSystemLibrary.MoveComponentTo` _p_tornado1 (+ (`SceneComponent.K2_GetComponentLocation` _capsulecomponent) (1000.0 1000.0 0.0)) (struct) false false 1.0)
          (`KismetSystemLibrary.MoveComponentTo` _p_tornado1 _returnvalue (struct) false false 0.0)
          (`SceneComponent.SetVisibility` _p_tornado1 false false))
        (:`then_2`
          (bind _p_tornado (`/Game/Game/Blueprints/Boss/BP_Boss.P_Tornado` _asbp_boss))
          (`SceneComponent.SetVisibility` _p_tornado true false)
          (`KismetSystemLibrary.MoveComponentTo` _p_tornado (+ (`SceneComponent.K2_GetComponentLocation` _capsulecomponent) (1000.0 0.0 0.0)) (struct) false false 1.0)
          (`KismetSystemLibrary.MoveComponentTo` _p_tornado _returnvalue (struct) false false 0.0)
          (`SceneComponent.SetVisibility` _p_tornado false false)))
      (set `/Game/Game/Blueprints/Boss/BP_Boss.TatsuFlag` false _asbp_boss)
      (else
        (`SceneComponent.SetVisibility` _p_tornado true false)
        (`KismetSystemLibrary.MoveComponentTo` _p_tornado (+ (5000.0 0.0 0.0) (`SceneComponent.K2_GetComponentLocation` _capsulecomponent)) (struct) true true 3.0)
        (`KismetSystemLibrary.MoveComponentTo` _p_tornado _returnvalue (struct) false false 0.0)
        (`SceneComponent.SetVisibility` _p_tornado false false)
        (set `/Game/Game/Blueprints/Boss/BP_Boss.TatsuFlag` false _asbp_boss)))
    (`self.FinishExecute` false)
    (else
      (`self.FinishExecute` true))))