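; Boss Blueprint that damages the player on contact, depending on the boss's current state.
; Mesh, Capsule and Sphere overlaps each act only in their own BossStates values, then check for a "Player" component tag and call DamageToPlayer on MyGameInstance.
; BeginPlay sets the initial state and stores the player pawn's location, which nothing here reads.
; Mesh overlaps also print the other actor's name.
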(event `self.ReceiveBeginPlay`
  (set `self.BossStates` "NewEnumerator8")
  (set `self.TargetPos` (`self.K2_GetActorLocation` (`GameplayStatics.GetPlayerPawn` 0))))

(event `self.ReceiveActorBeginOverlap`
  (params (OtherActor :type "Actor Object Reference")))

(event `self.ReceiveTick`
  (params (DeltaSeconds :type "Float (single-precision)")))

(event `self.Mesh.OnComponentBeginOverlap`
  (params (OverlappedComponent :type "PrimitiveComponent Object Reference") (OtherActor :type "Actor Object Reference") (OtherComp :type "PrimitiveComponent Object Reference") (OtherBodyIndex :type Integer) (bFromSweep :type Boolean) (SweepResult :type "HitResult Structure (by ref)"))
  (bind _bossstates (`self.BossStates`))
  (`KismetSystemLibrary.PrintString` (`KismetSystemLibrary.GetDisplayName` OtherActor))
  (if (`|EnumEquality` _bossstates "NewEnumerator5")
    (if (`ActorComponent.ComponentHasTag` OtherComp "Player") :!label _label
      (bind _asmy_game_instance (cast `MyGameInstance` (`GameplayStatics.GetGameInstance`)))
      (`MyGameInstance.DamageToPlayer` _asmy_game_instance 1.0))
    (elif (`|EnumEquality` _bossstates "NewEnumerator4")
      (goto _label))))

(event `self.Capsule.OnComponentBeginOverlap`
  (params (OverlappedComponent :type "PrimitiveComponent Object Reference") (OtherActor :type "Actor Object Reference") (OtherComp :type "PrimitiveComponent Object Reference") (OtherBodyIndex :type Integer) (bFromSweep :type Boolean) (SweepResult :type "HitResult Structure (by ref)"))
  (if (`|EnumEquality` (`self.BossStates`) "NewEnumerator2")
    (if (`ActorComponent.ComponentHasTag` OtherComp "Player")
      (bind _asmy_game_instance (cast `MyGameInstance` (`GameplayStatics.GetGameInstance`)))
      (`MyGameInstance.DamageToPlayer` _asmy_game_instance 1.0))))

(event `self.Sphere.OnComponentBeginOverlap`
  (params (OverlappedComponent :type "PrimitiveComponent Object Reference") (OtherActor :type "Actor Object Reference") (OtherComp :type "PrimitiveComponent Object Reference") (OtherBodyIndex :type Integer) (bFromSweep :type Boolean) (SweepResult :type "HitResult Structure (by ref)"))
  (if (`|EnumEquality` (`self.BossStates`) "NewEnumerator1")
    (if (`ActorComponent.ComponentHasTag` OtherComp "Player")
      (bind _asmy_game_instance (cast `MyGameInstance` (`GameplayStatics.GetGameInstance`)))
      (`MyGameInstance.DamageToPlayer` _asmy_game_instance 1.0))))

(fn `UserConstructionScript`)