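; BP_Player3 is a player Blueprint that drives two hand components from motion controllers, with threshold-filtered transform snapshots.
; Each Tick refreshes an MCTransform component when its controller's distance from world origin differs from the snapshot's by more than Changevalue.
; HandL follows its snapshot's location and rotation, while HandR follows the raw right controller, leaving MCTransformR unused for hand placement.
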(event `self.ReceiveBeginPlay`
  (`self.SetMotionControllerPosL`)
  (`self.SetMotionControllerPosR`))

(event `self.ReceiveTick`
  (params (DeltaSeconds :type "Float (single-precision)"))
  (bind _returnvalue_location (`KismetMathLibrary.BreakTransform` (`SceneComponent.K2_GetComponentToWorld` (`self.MC_Transform_L`))))
  (bind _returnvalue_location_2 (`KismetMathLibrary.BreakTransform` (`SceneComponent.K2_GetComponentToWorld` (`self.MotionController_L`))))
  (bind (_returnvalue_location_3 _returnvalue_rotation) (`KismetMathLibrary.BreakTransform` (`SceneComponent.K2_GetComponentToWorld` (`self.MC_Transform_L`))))
  (bind _returnvalue_location_4 (`KismetMathLibrary.BreakTransform` (`SceneComponent.K2_GetComponentToWorld` (`self.MC_Transform_R`))))
  (bind _returnvalue_location_5 (`KismetMathLibrary.BreakTransform` (`SceneComponent.K2_GetComponentToWorld` (`self.MotionController_R`))))
  (`|ExecutionSequence`
    (:`then_0`
      (if (> (`KismetMathLibrary.Abs` (- (`KismetMathLibrary.VSize` _returnvalue_location_2) (`KismetMathLibrary.VSize` _returnvalue_location))) (`self.Changevalue`))
        (`self.SetMotionControllerPosL`)))
    (:`then_1`
      (if (> (`KismetMathLibrary.Abs` (- (`KismetMathLibrary.VSize` _returnvalue_location_5) (`KismetMathLibrary.VSize` _returnvalue_location_4))) (`self.Changevalue`))
        (`self.SetMotionControllerPosR`)))
    (:`then_2`
      (`SceneComponent.K2_SetWorldTransform` (`self.handL`) (`KismetMathLibrary.MakeTransform` _returnvalue_location_3 _returnvalue_rotation) false false)
      (`SceneComponent.K2_SetWorldTransform` (`self.handR`) (`SceneComponent.K2_GetComponentToWorld` (`self.MotionController_R`)) false false))))

(fn `SetMotionControllerPosL`
  (`SceneComponent.K2_SetWorldTransform` (`self.MC_Transform_L`) (`SceneComponent.K2_GetComponentToWorld` (`self.MotionController_L`)) false false))

(fn `SetMotionControllerPosR`
  (`SceneComponent.K2_SetWorldTransform` (`self.MC_Transform_R`) (`SceneComponent.K2_GetComponentToWorld` (`self.MotionController_R`)) false false))

(fn `UserConstructionScript`)