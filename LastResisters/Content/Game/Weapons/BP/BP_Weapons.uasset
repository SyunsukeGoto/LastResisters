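; BP_Weapons is a katana actor for a motion-controller pawn that attaches to the right-hand socket and damages enemies when swung.
; While equipped, enemy overlap start plays spark and sound, and overlap end scales damage by swing distance for BP_Boss or BP_Enemy1 in specific states.
; Hits drain durability until the weapon breaks and is removed, with Remove hiding the mesh far below.
; While unequipped, Tick restores durability after a delay.
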(event `self.ReceiveBeginPlay`
  (bind _staticmeshcomponent (`self.StaticMeshComponent`))
  (bind _output_get (set `self.WepansModelArray` (`|MakeArray` "/Game/Game/Weapons/FBX/Katana/SM_Katana.SM_Katana" :!type "StaticMesh Object Reference")))
  (`StaticMeshComponent.SetStaticMesh` _staticmeshcomponent (`|GetArrayItem` _output_get))
  (`PrimitiveComponent.SetSimulatePhysics` _staticmeshcomponent false))

(event `self.ReceiveTick`
  (params (DeltaSeconds :type "Float (single-precision)"))
  (if (not (`self.UseFlag`))
    (`KismetSystemLibrary.Delay` 5.0)
    (set `self.DurableValue` 100)
    (set `self.IsBreak` false)))

(event `/Game/VirtualRealityBP/Blueprints/PickupActorInterface.Equip`
  (params (AttachTo :type "SceneComponent Object Reference") (DominantHand :type "EControllerHand Enum" :default "Left"))
  (bind _staticmeshcomponent (`self.StaticMeshComponent`))
  (`PrimitiveComponent.SetSimulatePhysics` _staticmeshcomponent false)
  (`self.K2_DetachFromActor` "KeepWorld" "KeepWorld" "KeepWorld")
  (`SceneComponent.K2_AttachToComponent` (`self.K2_GetRootComponent`) AttachTo "RightHandPosition" "KeepWorld" "KeepWorld" "KeepWorld" false)
  (`SceneComponent.K2_SetRelativeLocationAndRotation` _staticmeshcomponent (0.8 2.5 -0.6) (struct :`Pitch` 60.0 :`Yaw` -70.0 :`Roll` 15.0) false false)
  (set `self.UseFlag` true))

(event `/Game/VirtualRealityBP/Blueprints/PickupActorInterface.Remove`
  (params (AttachTo :type "SceneComponent Object Reference"))
  (bind (_returnvalue_x _returnvalue_y _returnvalue_z) (`KismetMathLibrary.BreakVector` (`SceneComponent.K2_GetComponentLocation` AttachTo)))
  (`PrimitiveComponent.SetSimulatePhysics` (`self.StaticMeshComponent`) false)
  (`self.K2_DetachFromActor` "KeepWorld" "KeepWorld" "KeepWorld")
  (`SceneComponent.K2_AttachToComponent` (`self.K2_GetRootComponent`) AttachTo "RightHandPosition" "KeepWorld" "KeepWorld" "KeepWorld" false)
  (`SceneComponent.K2_SetRelativeLocationAndRotation` (`self.StaticMeshComponent`) (`KismetMathLibrary.MakeVector` _returnvalue_x _returnvalue_y (- _returnvalue_z 10000.0)) (struct :`Pitch` 90.0 :`Roll` 90.0) false false)
  (set `self.UseFlag` false))

(event `self.StaticMeshComponent.OnComponentBeginOverlap`
  (params (OverlappedComponent :type "PrimitiveComponent Object Reference") (OtherActor :type "Actor Object Reference") (OtherComp :type "PrimitiveComponent Object Reference") (OtherBodyIndex :type Integer) (bFromSweep :type Boolean) (SweepResult :type "HitResult Structure (by ref)"))
  (bind _returnvalue (`SceneComponent.K2_GetComponentLocation` (`self.Scene`)))
  (if (`self.UseFlag`)
    (if (`ActorComponent.ComponentHasTag` (`.HitComponent` (`GameplayStatics.BreakHitResult` SweepResult)) "Enemy")
      (`GameplayStatics.SpawnEmitterAtLocation` "/Game/Game/Effect/SparkEffect/P_sparkEffectType003.P_sparkEffectType003" _returnvalue)
      (set `self.BeginPos` _returnvalue)
      (`GameplayStatics.PlaySoundAtLocation` "/Game/Game/Sound/SE/Attack.Attack" _returnvalue (struct) 1.0 1.0 0.0 null null null))))

(event `self.StaticMeshComponent.OnComponentEndOverlap`
  (params (OverlappedComponent :type "PrimitiveComponent Object Reference") (OtherActor :type "Actor Object Reference") (OtherComp :type "PrimitiveComponent Object Reference") (OtherBodyIndex :type Integer))
  (if (`self.UseFlag`)
    (if (`self.ActorHasTag` OtherActor "Enemy")
      (bind _output_get (set `self.EndPos` (`SceneComponent.K2_GetComponentLocation` (`self.StaticMeshComponent`))))
      (bind _distance (`/Game/VirtualRealityBP/Blueprints/FunctionLibrary.GetDistance_Vector3` (`self.BeginPos`) _output_get))
      (bind _damage (`self.DamageCalculation` _distance))
      (bind _asbp_boss (cast `/Game/Game/Blueprints/Boss/BP_Boss` OtherActor)
        (:`then`
          (if (`|EnumEquality` (`/Game/Game/Blueprints/Boss/BP_Boss.BossStates` _asbp_boss) "NewEnumerator0")
            (if (`self.UseFlag`)
              (set `/Game/Game/Blueprints/Boss/BP_Boss.Hp` (- (`/Game/Game/Blueprints/Boss/BP_Boss.Hp` _asbp_boss) (`KismetMathLibrary.FTrunc` (/ _damage 4.0))) _asbp_boss)
              ;[1 1 1] Initialization
              (`self.ReduceDurableValue`)
              (set `self.BeginPos` (0.0 0.0 0.0) :!label _label)
              (set `self.EndPos` (0.0 0.0 0.0)))))
        (:`CastFailed`
          (bind _asbp_enemy_1 (cast `/Game/Game/Blueprints/Enemy/Enemy1/BP_Enemy1` OtherActor)
            (:`then`
              (if (`|EnumEquality` (`/Game/Game/Blueprints/Enemy/Enemy1/BP_Enemy1.Enemy1State` _asbp_enemy_1) "NewEnumerator4")
                (if (`self.UseFlag`)
                  (set `/Game/Game/Blueprints/Enemy/Enemy1/BP_Enemy1.Hp` (- (`/Game/Game/Blueprints/Enemy/Enemy1/BP_Enemy1.Hp` _asbp_enemy_1) (`KismetMathLibrary.FTrunc` (/ _damage 2.0))) _asbp_enemy_1)
                  (`self.ReduceDurableValue`)
                  (goto _label))))
            (:`CastFailed`
              (goto _label))))))))

(fn `DamageCalculation`
  (params (distance :type "Float (double-precision)"))
  (returns (Damage :type "Float (double-precision)"))
  (return (* (/ distance (`self.Max Dist`)) (`self.Damage`))))

(fn `ReduceDurableValue`
  (bind _returnvalue (- (`self.DurableValue`) 10))
  (if (`self.UseFlag`)
    (if (<= _returnvalue 0)
      (message `/Game/VirtualRealityBP/Blueprints/PickupActorInterface.Remove` self (`Character.Mesh` (cast `/Game/VirtualRealityBP/Blueprints/MotionControllerPawn` (`GameplayStatics.GetPlayerPawn` 0) :!pure true)))
      (set `self.DurableValue` 0)
      (set `self.IsBreak` true)
      (`GameplayStatics.PlaySoundAtLocation` "/Game/Game/Sound/SE/BreakWeapon.BreakWeapon" (`SceneComponent.K2_GetComponentLocation` (`self.StaticMeshComponent`)) (struct) 1.0 1.0 0.0 null null null)
      (else
        (set `self.DurableValue` _returnvalue)))))

(fn `UserConstructionScript`)