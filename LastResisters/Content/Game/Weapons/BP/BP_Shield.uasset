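; Shield weapon actor that can be held in a hand or stowed on another component, and shows sparks on a guard.
; Equip and Remove reattach it to the given component with preset mesh offsets, setting UseShieldFlag for a left dominant hand and clearing it on removal.
; Tick polls MyGameInstance's guard flag, reports the effect as spawned, and emits sparks beside the mesh.
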(event `self.ReceiveBeginPlay`
  (bind _staticmeshcomponent (`self.StaticMeshComponent`))
  (bind _output_get (set `self.ShieldsModelArray` (`|MakeArray` "/Game/Game/Weapons/FBX/Shield/SM_Shield.SM_Shield" :!type "StaticMesh Object Reference")))
  (`StaticMeshComponent.SetStaticMesh` _staticmeshcomponent (`|GetArrayItem` _output_get))
  (`PrimitiveComponent.SetSimulatePhysics` _staticmeshcomponent false))

(event `/Game/VirtualRealityBP/Blueprints/PickupActorInterface.Equip`
  (params (AttachTo :type "SceneComponent Object Reference") (DominantHand :type "EControllerHand Enum" :default "Left"))
  (bind _staticmeshcomponent (`self.StaticMeshComponent`))
  (`PrimitiveComponent.SetSimulatePhysics` _staticmeshcomponent false)
  (`self.K2_DetachFromActor` "KeepWorld" "KeepWorld" "KeepWorld")
  (`SceneComponent.K2_AttachToComponent` (`self.K2_GetRootComponent`) AttachTo "None" "KeepWorld" "KeepWorld" "KeepWorld" false)
  (if (`|EnumEquality` DominantHand "Left")
    (`SceneComponent.K2_SetRelativeLocationAndRotation` _staticmeshcomponent (0.0 0.0 0.0) (struct :`Pitch` -90.0 :`Roll` 180.0) false false)
    (set `self.UseShieldFlag` true)
    (else
      (`SceneComponent.K2_SetRelativeLocationAndRotation` _staticmeshcomponent (0.0 0.0 0.0) (struct :`Pitch` 90.0) false false))))

(event `/Game/VirtualRealityBP/Blueprints/PickupActorInterface.Remove`
  (params (AttachTo :type "SceneComponent Object Reference"))
  (`PrimitiveComponent.SetSimulatePhysics` (`self.StaticMeshComponent`) false)
  (`self.K2_DetachFromActor` "KeepWorld" "KeepWorld" "KeepWorld")
  (`SceneComponent.K2_AttachToComponent` (`self.K2_GetRootComponent`) AttachTo "None" "KeepWorld" "KeepWorld" "KeepWorld" false)
  (`SceneComponent.K2_SetRelativeLocationAndRotation` (`self.StaticMeshComponent`) (-20.0 0.0 30.0) (struct :`Pitch` 90.0 :`Roll` 90.0) false false)
  (set `self.UseShieldFlag` false))

(event `self.ReceiveTick`
  (params (DeltaSeconds :type "Float (single-precision)"))
  (bind _staticmeshcomponent (`self.StaticMeshComponent`))
  ;[1 1 1] Spawn Emitter Guard
  (bind _asmy_game_instance (cast `MyGameInstance` (`GameplayStatics.GetGameInstance`)))
  (bind _returnvalue (`MyGameInstance.GetIfGuard` _asmy_game_instance))
  (if _returnvalue
    (`MyGameInstance.GuardEffectSpawned` _asmy_game_instance)
    (`GameplayStatics.SpawnEmitterAtLocation` "/Game/Game/Effect/SparkEffect/P_sparkEffectType003.P_sparkEffectType003" (+ (`SceneComponent.K2_GetComponentLocation` _staticmeshcomponent) (* (`SceneComponent.GetRightVector` _staticmeshcomponent) 20.0)) (struct) (0.25 0.25 0.25))))

(fn `UserConstructionScript`)