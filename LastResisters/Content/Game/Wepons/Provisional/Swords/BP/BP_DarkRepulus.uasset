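; BP_DarkRepulus is a provisional sword weapon that switches between an equipped and a removed placement.
; Equip disables mesh physics, attaches the root to the supplied component and applies a fixed relative offset and rotation to the mesh.
; Remove re-enables physics, detaches the actor, then makes another attach call to the supplied component and sets a different mesh transform, apparently a stowed pose.
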(event `/Game/VirtualRealityBP/Blueprints/PickupActorInterface.Equip`
  (params (AttachTo :type "SceneComponent Object Reference"))
  (bind _staticmeshcomponent (`self.StaticMeshComponent`))
  (`PrimitiveComponent.SetSimulatePhysics` _staticmeshcomponent false)
  (`SceneComponent.K2_AttachToComponent` (`self.K2_GetRootComponent`) AttachTo "None" "KeepWorld" "KeepWorld" "KeepWorld" false)
  (`SceneComponent.K2_SetRelativeLocationAndRotation` _staticmeshcomponent (-3.0 0.0 0.0) (struct :`Pitch` -90.0) false false))

(event `/Game/VirtualRealityBP/Blueprints/PickupActorInterface.Remove`
  (params (AttachTo :type "SceneComponent Object Reference"))
  (bind _staticmeshcomponent (`self.StaticMeshComponent`))
  (`PrimitiveComponent.SetSimulatePhysics` _staticmeshcomponent true)
  (`self.K2_DetachFromActor` "KeepWorld" "KeepWorld" "KeepWorld")
  (`self.K2_AttachToComponent` AttachTo "None" "KeepRelative" "KeepRelative" "KeepRelative")
  (`SceneComponent.K2_SetRelativeLocationAndRotation` _staticmeshcomponent (-20.0 0.0 -30.0) (struct :`Pitch` -80.0 :`Yaw` 90.0) false false))

(fn `UserConstructionScript`)